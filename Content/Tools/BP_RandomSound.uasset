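; BP_RandomSound is a trigger-zone actor that plays a sound at random positions around the third-person character inside it.
; On BeginPlay it spawns a box, capsule or sphere trigger chosen by enum and binds its overlap events.
; Entry starts a looping timer that plays the sound at random per-axis offsets from the character; exit clears it.
; Each sound also spawns a BP_Debug actor at its location, destroyed immediately.
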(event Custom|BeginOverlap
  (params (OverlappedActor :type Actor%20Object%20Reference) (OtherActor :type Actor%20Object%20Reference))
  (bind _asbp_third_person_character (Utilities|Casting|CastToBP_ThirdPersonCharacter OtherActor))
  (Variables|Default|SetCharacterRef _asbp_third_person_character)
  (CallFunction|StartRandomSound))

(event Custom|EndOverlap
  (params (OverlappedActor :type Actor%20Object%20Reference) (OtherActor :type Actor%20Object%20Reference))
  (Utilities|Casting|CastToBP_ThirdPersonCharacter OtherActor)
  (Utilities|Time|ClearandInvalidateTimerbyHandle (Variables|Default|GetTimerHandler)))

(event Custom|StartRandomSound
  (bind _returnvalue (Utilities|Time|SetTimerbyEvent (delegate Custom|RandomSoundSpawn) (Variables|Default|GetTimeSound) true))
  (Variables|Default|SetTimerHandler _returnvalue))

(event Custom|RandomSoundSpawn
  (bind _characterref (Variables|Default|GetCharacterRef))
  (bind _minrange (Variables|Default|GetMinRange))
  (bind _maxrange (Variables|Default|GetMaxRange))
  (bind _returnvalue (Transformation|GetActorLocation _characterref))
  (bind _returnvalue_2 (Math|Random|RandomFloatinRange _minrange _maxrange))
  (bind _returnvalue_3 (Audio|SpawnSoundatLocation "/Game/Sounds/KasaneTeto.KasaneTeto" (Math|Vector|MakeVector (+ (.x _returnvalue) _returnvalue_2) (+ (.y _returnvalue) _returnvalue_2) (+ (.z _returnvalue) _returnvalue_2)) "0, 0, 0" 1.0 1.0 0.0 0 0))
  (bind _returnvalue_4 (Game|SpawnActorfromClass "/Game/Blueprints/BP_Debug.BP_Debug_C" (Math|Transform|MakeTransform (Transformation|GetWorldLocation _returnvalue_3) "0, 0, 0" "1.000000,1.000000,1.000000") "AlwaysSpawn" "MultiplyWithRoot" 0 0))
  (Rendering|SetActorHiddenInGame _returnvalue_4 false)
  (Actor|DestroyActor _returnvalue_4))

(event EventBeginPlay
  (bind _defaultsceneroot (Variables|Default|GetDefaultSceneRoot))
  (bind _returnvalue (Transformation|GetWorldTransform _defaultsceneroot))
  (bind _returnvalue_2 (Game|SpawnActorfromClass (Utilities|Select :Index (Variables|Default|GetERef) :NewEnumerator0 "/Script/Engine.TriggerBox" :NewEnumerator1 "/Script/Engine.TriggerCapsule" :NewEnumerator2 "/Script/Engine.TriggerSphere") (Math|Transform|MakeTransform (.location _returnvalue) (.rotation _returnvalue) (Variables|Default|GetScale)) "Undefined" "MultiplyWithRoot" 0 0))
  (Rendering|SetActorHiddenInGame _returnvalue_2 false)
  (Collision|BindEventtoOnActorBeginOverlap _returnvalue_2 (delegate Custom|BeginOverlap))
  (Collision|BindEventtoOnActorEndOverlap _returnvalue_2 (delegate Custom|EndOverlap)))

(fn ConstructionScript)