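; BP_River is a river actor that keeps a spawned BP_Sound emitter on the point of its spline nearest the player.
; On BeginPlay it caches the third-person character, spawns the sound actor at the spline and starts a fast looping timer.
; Each timer tick moves the sound to the closest spline point, but only while the player is within MaxDistance of the spline, so one emitter covers the river.
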(event Custom|UpdateSoundLocation
  (if (<= (Math|Vector|VectorLength (- (Spline|FindLocationClosesttoWorldLocation (Variables|Default|GetSpline) (Transformation|GetActorLocation (Variables|Default|GetCharacterRef)) "World") (Transformation|GetActorLocation (Variables|Default|GetCharacterRef)))) (Variables|Default|GetMaxDistance))
    (Transformation|SetWorldLocation (Variables|/Game/Blueprints/BP_Sound.BP_Sound_C|GetDefaultSceneRoot (Variables|Default|GetSoundRef)) (Spline|FindLocationClosesttoWorldLocation (Variables|Default|GetSpline) (Transformation|GetActorLocation (Variables|Default|GetCharacterRef)) "World") false false)))

(event EventBeginPlay
  (Utilities|FlowControl|Sequence
    (:then_0
      (bind _asbp_third_person_character (Utilities|Casting|CastToBP_ThirdPersonCharacter (Game|GetPlayerCharacter 0)))
      (Variables|Default|SetCharacterRef _asbp_third_person_character))
    (:then_1
      (bind _returnvalue (Game|SpawnActorfromClass "/Game/Blueprints/BP_Sound.BP_Sound_C" (Math|Transform|MakeTransform (Transformation|GetWorldLocation (Variables|Default|GetSpline)) "0, 0, 0" "1.000000,1.000000,1.000000") "Undefined" "MultiplyWithRoot" 0 0))
      (Variables|Default|SetSoundRef _returnvalue))
    (:then_2
      (Utilities|Time|SetTimerbyEvent (delegate Custom|UpdateSoundLocation) 0.01 true))))

(fn ConstructionScript)